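; Thrown bottle projectile that ragdolls the third-person character it overlaps, with an effect depending on its bottle type.
; On spawn it boosts its velocity with an upward lob, then enables sphere overlaps after a short delay.
; Water lowers the target's drunk variable and ragdolls briefly, while alcohol only ragdolls for longer; already ragdolled characters are ignored.
; It destroys itself after affecting a character or when its mesh hits anything else.
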(event OnComponentHit(StaticMesh)
  (params (HitComponent :type Primitive%20Component%20Object%20Reference) (OtherActor :type Actor%20Object%20Reference) (OtherComp :type Primitive%20Component%20Object%20Reference) (NormalImpulse :type Vector :default "0, 0, 0") (Hit :type Hit%20Result%20Structure%20%28by%20ref%29))
  (Utilities|Casting|CastToBP_ThirdPersonCharacter OtherActor
    (:CastFailed
      (Actor|DestroyActor))))

(event OnComponentBeginOverlap(Sphere)
  (params (OverlappedComponent :type Primitive%20Component%20Object%20Reference) (OtherActor :type Actor%20Object%20Reference) (OtherComp :type Primitive%20Component%20Object%20Reference) (OtherBodyIndex :type Integer) (bFromSweep :type Boolean) (SweepResult :type Hit%20Result%20Structure%20%28by%20ref%29))
  (bind _asbp_third_person_character (Utilities|Casting|CastToBP_ThirdPersonCharacter OtherActor))
  (CallFunction|SobertyIsLiberty _asbp_third_person_character))

(event Custom|SobertyIsLiberty
  (params (Actor :type BP%20Third%20Person%20Character%20Object%20Reference))
  (if (not (Variables|/Game/BP/ETHYLORUN/BP_ThirdPersonCharacter.BP_ThirdPersonCharacter_C|GetRagdoll Actor))
    (switch Utilities|FlowControl|Switch|SwitchonEnum_BottleType (Variables|Default|GetBottleType)
      (:NewEnumerator0
        (Variables|/Game/BP/ETHYLORUN/BP_ThirdPersonCharacter.BP_ThirdPersonCharacter_C|SetDrunkVariable Actor (- (Variables|/Game/BP/ETHYLORUN/BP_ThirdPersonCharacter.BP_ThirdPersonCharacter_C|GetDrunkVariable Actor) 0.25))
        (Default|RagdollEvent Actor 2.0))
      (:NewEnumerator1
        (Default|RagdollEvent Actor 4.0)))
    (Actor|DestroyActor)))

(event Custom|GetWaterType
  (params (NewParam :type Enum_BottleType%20Enum :default "NewEnumerator0"))
  (Variables|Default|SetBottleType NewParam))

(event EventBeginPlay
  (bind _returnvalue (Transformation|GetVelocity))
  (Game|Components|ProjectileMovement|SetVelocityinLocalSpace (Variables|Default|GetProjectileMovement) (Math|Vector|MakeVector (* (.x _returnvalue) 2.0) (* (.y _returnvalue) 2.0) 5e+02))
  (Utilities|FlowControl|Delay 0.1)
  (Variables|/Script/Engine.PrimitiveComponent|SetbGenerateOverlapEvents (Variables|Default|GetSphere) true))

(event Collision|EventActorBeginOverlap
  (params (OtherActor :type Actor%20Object%20Reference)))

(event EventTick
  (params (DeltaSeconds :type Float%20%28single-precision%29)))

(fn ConstructionScript)