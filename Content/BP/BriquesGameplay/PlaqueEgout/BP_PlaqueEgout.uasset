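; Manhole cover hazard that cycles between calm, wobbling, rising on a geyser-like Niagara effect and dropping back down.
; Idle and Lunch timelines chain through FlipFlops, wobbling the cover, then alternately raising or lowering it with the effect and capsule.
; The capsule launches and ragdolls overlapping characters and impulses other components.
; Their collision on GameTraceChannel1 is ignored until the next idle phase restores it.
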(event OnComponentBeginOverlap(Capsule)
  (params (OverlappedComponent :type Primitive%20Component%20Object%20Reference) (OtherActor :type Actor%20Object%20Reference) (OtherComp :type Primitive%20Component%20Object%20Reference) (OtherBodyIndex :type Integer) (bFromSweep :type Boolean) (SweepResult :type Hit%20Result%20Structure%20%28by%20ref%29))
  (bind _returnvalue (Transformation|GetActorForwardVector))
  (bind _returnvalue_2 (Transformation|GetActorForwardVector))
  (bind _returnvalue_3 (* _returnvalue_2 5e+02))
  (bind _asbp_third_person_character (Utilities|Casting|CastToBP_ThirdPersonCharacter OtherActor)
    (:then
      (Variables|Default|SetAs%20BP%20Third%20Person%20Character _asbp_third_person_character)
      (Character|LaunchCharacter (Variables|Default|GetAs%20BP%20Third%20Person%20Character) (Math|Vector|MakeVector (.x _returnvalue_3) (.y _returnvalue_3) 5e+02) false false)
      (Utilities|Array|Add (Variables|Default|GetThird%20Person%20Character%20Array) (Variables|Default|GetAs%20BP%20Third%20Person%20Character))
      (Collision|SetCollisionResponsetoChannel (Variables|/Script/Engine.Character|GetCapsuleComponent (Variables|Default|GetAs%20BP%20Third%20Person%20Character)) "ECC_GameTraceChannel1" "ECR_Ignore")
      (Utilities|FlowControl|Delay 0.2)
      (Default|RagdollEvent (Variables|Default|GetAs%20BP%20Third%20Person%20Character) 3.0))
    (:CastFailed
      (bind _output_get (Variables|Default|SetTouchedComp OtherComp))
      (Utilities|IsValid _output_get
        (:Is%20Valid
          (Physics|AddImpulse OtherComp (Math|Vector|MakeVector (* (.x _returnvalue) 2.5e+02) (* (.y _returnvalue) 2.5e+02) 5e+02) "None" true)
          (Utilities|Array|Add (Variables|Default|GetTouchedComps) (Variables|Default|GetTouchedComp))
          (Collision|SetCollisionResponsetoChannel (Variables|Default|GetTouchedComp) "ECC_GameTraceChannel1" "ECR_Ignore"))))))

(event Custom|Start%20Idle
  (bind _touchedcomps (Variables|Default|GetTouchedComps))
  (Utilities|FlowControl|Sequence
    (:then_0
      (Utilities|FlowControl|FlipFlop
        (:A
          (Utilities|FlowControl|Delay (Variables|Default|GetCalmTime))
          (bind (_direction _xrotate _yrotate) (Timeline|Idle PlayFromStart)
            (:Update
              (Transformation|SetWorldRotation (Variables|Default|GetPlaque) (Math|Rotator|MakeRotator _xrotate _yrotate 0.0) false false))
            (:Finished
              (Utilities|FlowControl|FlipFlop
                (:A
                  (CallFunction|StartLunch))
                (:B
                  (CallFunction|EndLunch))))))
        (:B
          (Timeline|Idle PlayFromStart))))
    (:then_1
      (for _array_element _touchedcomps
        (Collision|SetCollisionResponsetoChannel _array_element "ECC_GameTraceChannel1" "ECR_Block"))
      (Utilities|Array|Clear _touchedcomps)
      (for _array_element_2 (Variables|Default|GetThird%20Person%20Character%20Array)
        (Collision|SetCollisionResponsetoChannel (Variables|/Script/Engine.Character|GetCapsuleComponent _array_element_2) "ECC_GameTraceChannel1" "ECR_Block"))
      (Utilities|Array|Clear (Variables|Default|GetThird%20Person%20Character%20Array)))))

(event Custom|Start%20Lunch
  (Collision|SetCollisionEnabled (Variables|Default|GetCapsule) "QueryAndPhysics")
  (Variables|/Script/Engine.PrimitiveComponent|SetbGenerateOverlapEvents (Variables|Default|GetCapsule) true)
  (bind _z_location (Timeline|Lunch PlayFromStart)
    (:Update
      (Transformation|SetRelativeLocation (Variables|Default|GetPlaque) (Math|Vector|MakeVector 0.0 0.0 (* _z_location 275.0)) false false)
      (Transformation|SetRelativeLocation (Variables|Default|GetNiagara) (Math|Vector|MakeVector 0.0 0.0 (- (* _z_location 275.0) 275.0)) false false)
      (Transformation|SetRelativeLocation (Variables|Default|GetCapsule) (Math|Vector|MakeVector 0.0 0.0 (- (* _z_location 275.0) 1.4e+02)) false false))
    (:Finished
      (CallFunction|StartIdle))))

(event Custom|End%20Lunch
  (Collision|SetCollisionEnabled (Variables|Default|GetCapsule) "NoCollision")
  (Variables|/Script/Engine.PrimitiveComponent|SetbGenerateOverlapEvents (Variables|Default|GetCapsule) false)
  (bind _z_location (Timeline|Lunch ReverseFromEnd)
    (:Update
      (Transformation|SetRelativeLocation (Variables|Default|GetPlaque) (Math|Vector|MakeVector 0.0 0.0 (* _z_location 275.0)) false false)
      (Transformation|SetRelativeLocation (Variables|Default|GetNiagara) (Math|Vector|MakeVector 0.0 0.0 (- (* _z_location 275.0) 275.0)) false false)
      (Transformation|SetRelativeLocation (Variables|Default|GetCapsule) (Math|Vector|MakeVector 0.0 0.0 (- (* _z_location 275.0) 1.4e+02)) false false))
    (:Finished
      (CallFunction|StartIdle))))

(event EventBeginPlay
  (CallFunction|StartIdle))

(fn ConstructionScript)