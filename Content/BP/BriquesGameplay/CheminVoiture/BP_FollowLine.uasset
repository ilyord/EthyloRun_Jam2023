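; BP_FollowLine is a car-path actor that continuously spawns vehicles to travel along it.
; From BeginPlay, SpawnLoop waits a random delay between its min and max rates, spawns a random class from VehicleEnable, then calls itself again.
; Each vehicle spawns at the root's location, receives this actor as SplineToFollow along with the travel time, and starts moving through its own MoveObject.
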(event Custom|Spawn%20Vehicle
  (params (Class :type BP%20Vehicle%20Class%20Reference))
  (bind _returnvalue (Game|SpawnActorfromClass Class (Math|Transform|MakeTransform (Transformation|GetWorldLocation (Variables|Default|GetDefaultSceneRoot)) "0, 0, 0" "1.000000,1.000000,1.000000") "Undefined" 0 0))
  (Variables|/Game/BP/BriquesGameplay/CheminVoiture/BP_Vehicle.BP_Vehicle_C|SetSplineToFollow _returnvalue self)
  (Variables|/Game/BP/BriquesGameplay/CheminVoiture/BP_Vehicle.BP_Vehicle_C|SetTime%20To%20Complete%20%28%20in%20s%20%29 _returnvalue (Variables|Default|GetTime%20to%20Complete%20%28%20In%20S%20%29))
  (Default|MoveObject _returnvalue))

(event Custom|Spawn%20Loop
  (Utilities|FlowControl|Delay (Math|Random|RandomFloatinRange (Variables|Default|GetSpawn%20Rate%20Min%20%28%20in%20s%20%29) (Variables|Default|GetSpawn%20Rate%20Max%20%28%20in%20s%20%29)))
  (bind _random_vehicle (CallFunction|RandomizeVehicle))
  (CallFunction|SpawnVehicle _random_vehicle)
  (CallFunction|SpawnLoop))

(event EventBeginPlay
  (CallFunction|SpawnLoop))

(fn ConstructionScript)

(fn RandomizeVehicle
  (bind _output_get (Variables|Default|SetVehicle%20To%20Spawn (.OutItem (Utilities|Array|Random (Variables|Default|GetVehicle%20Enable)))))
  (return _output_get))