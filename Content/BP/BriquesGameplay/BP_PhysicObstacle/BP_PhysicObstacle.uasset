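; BP_PhysicObstacle is an obstacle actor that represents one of several street props, such as a bin, cone, table, chair, parasol or electric scooter.
; Its construction script switches on the Type variable to assign the matching static mesh, with the scooter using Shape_Pipe_180, apparently a placeholder.
; The event graph holds only disabled default events, so the Blueprint adds no runtime logic.
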(event EventBeginPlay)

(event Collision|EventActorBeginOverlap
  (params (OtherActor :type Actor%20Object%20Reference)))

(event EventTick
  (params (DeltaSeconds :type Float%20%28single-precision%29)))

(fn ConstructionScript
  (switch Utilities|FlowControl|Switch|SwitchonEnum_PhysicObstacleType (Variables|Default|GetType)
    (:NewEnumerator0
      (Components|StaticMesh|SetStaticMesh (Variables|Default|GetStaticMesh) "/Game/Props/Poubelle/Poubelle.Poubelle"))
    (:NewEnumerator1
      (Components|StaticMesh|SetStaticMesh (Variables|Default|GetStaticMesh) "/Game/Props/Cone/Cone.Cone"))
    (:NewEnumerator2
      (Components|StaticMesh|SetStaticMesh (Variables|Default|GetStaticMesh) "/Game/Props/ChaiseTable/Table.Table"))
    (:NewEnumerator3
      (Components|StaticMesh|SetStaticMesh (Variables|Default|GetStaticMesh) "/Game/Props/ChaiseTable/Chaise.Chaise"))
    (:NewEnumerator5
      (Components|StaticMesh|SetStaticMesh (Variables|Default|GetStaticMesh) "/Game/Props/ChaiseTable/Parassol.Parassol"))
    (:NewEnumerator4
      (Components|StaticMesh|SetStaticMesh (Variables|Default|GetStaticMesh) "/Game/StarterContent/Shapes/Shape_Pipe_180.Shape_Pipe_180"))))