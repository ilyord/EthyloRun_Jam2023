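; BP_Vent is a wind vent volume that pushes third-person characters along the forward direction of its box.
; Overlap events keep an array of the characters inside, with a flag that clears once it empties.
; Each tick, every tracked character gets a movement component force plus a weaker force on mesh bodies below spine_01, affecting any simulated physics bodies.
; The construction script sizes the box from a BoxExtent variable.
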(event OnComponentBeginOverlap(Box)
  (params (OverlappedComponent :type Primitive%20Component%20Object%20Reference) (OtherActor :type Actor%20Object%20Reference) (OtherComp :type Primitive%20Component%20Object%20Reference) (OtherBodyIndex :type Integer) (bFromSweep :type Boolean) (SweepResult :type Hit%20Result%20Structure%20%28by%20ref%29))
  (bind _asbp_third_person_character (Utilities|Casting|CastToBP_ThirdPersonCharacter OtherActor))
  (Utilities|Array|Add (Variables|Default|GetAs%20BP%20Third%20Person%20Character) _asbp_third_person_character)
  (Variables|Default|SetInBox true))

(event OnComponentEndOverlap(Box)
  (params (OverlappedComponent :type Primitive%20Component%20Object%20Reference) (OtherActor :type Actor%20Object%20Reference) (OtherComp :type Primitive%20Component%20Object%20Reference) (OtherBodyIndex :type Integer))
  (bind _as_bp_third_person_character (Variables|Default|GetAs%20BP%20Third%20Person%20Character))
  (bind _asbp_third_person_character (Utilities|Casting|CastToBP_ThirdPersonCharacter OtherActor))
  (Utilities|Array|RemoveItem _as_bp_third_person_character _asbp_third_person_character)
  (if (== (Utilities|Array|Length _as_bp_third_person_character) 0)
    (Variables|Default|SetInBox false)))

(event EventTick
  (params (DeltaSeconds :type Float%20%28single-precision%29))
  (bind _box (Variables|Default|GetBox))
  (bind _returnvalue (Math|Vector|GetForwardVector _box))
  (if (Variables|Default|GetInBox)
    (for _array_element (Variables|Default|GetAs%20BP%20Third%20Person%20Character)
      (Physics|AddForce (Variables|/Script/Engine.Character|GetCharacterMovement _array_element) (* _returnvalue 1.5e+05))
      (Class|SkeletalMeshComponent|AddForcetoAllBodiesBelow (Variables|/Script/Engine.Character|GetMesh _array_element) (* _returnvalue 1e+04) "spine_01" false false))))

(fn ConstructionScript
  (Components|Box|SetBoxExtent (Variables|Default|GetBox) (Variables|Default|GetBox%20Extent) true))