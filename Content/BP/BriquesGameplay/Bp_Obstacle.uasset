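; Configurable obstacle actor from the gameplay bricks, with a type choice of tree, blank, barrier or fire hydrant.
; The construction script assigns a basic-shape mesh and a box extent from the chosen type; only the tree gets a non-zero box by default.
; An override flag replaces that extent with a custom BoxCollision size.
; The event graph holds no active logic.
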(event EventBeginPlay)

(event Collision|EventActorBeginOverlap
  (params (OtherActor :type Actor%20Object%20Reference)))

(event EventTick
  (params (DeltaSeconds :type Float%20%28single-precision%29)))

(fn ConstructionScript
  (switch Utilities|FlowControl|Switch|SwitchonEnum_ObstacleType (Variables|Default|GetType)
    (:NewEnumerator0
      (Components|StaticMesh|SetStaticMesh (Variables|Default|GetStaticMesh) "/Game/StarterContent/Shapes/Shape_Cone.Shape_Cone")
      (Components|Box|SetBoxExtent (Variables|Default|GetBox) "100.000000,100.000000,300.000000" true))
    (:NewEnumerator1
      (Components|StaticMesh|SetStaticMesh (Variables|Default|GetStaticMesh) "/Game/StarterContent/Shapes/Shape_Cube.Shape_Cube")
      (Components|Box|SetBoxExtent (Variables|Default|GetBox) "0, 0, 0" true))
    (:NewEnumerator2
      (Components|StaticMesh|SetStaticMesh (Variables|Default|GetStaticMesh) "/Game/StarterContent/Props/MaterialSphere.MaterialSphere")
      (Components|Box|SetBoxExtent (Variables|Default|GetBox) "0, 0, 0" true))
    (:NewEnumerator3
      (Components|StaticMesh|SetStaticMesh (Variables|Default|GetStaticMesh) "/Game/StarterContent/Shapes/Shape_Pipe_180.Shape_Pipe_180")
      (Components|Box|SetBoxExtent (Variables|Default|GetBox) "0, 0, 0" true)))
  (if (Variables|Default|GetOverrightBoxSize)
    (Components|Box|SetBoxExtent (Variables|Default|GetBox) (Variables|Default|GetBoxCollision) true)))