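; BP_VoiturePolice is a police car actor that can knock the player character into a ragdoll when touched.
; When a BP_ThirdPersonCharacter overlaps its Box, the car launches it upward and along the character's own forward vector, then calls that character's RagdollEvent.
; The construction script enables the Box's overlap events only when the RagdollEffect flag is set, so each instance can turn the effect on or off.
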(event OnComponentBeginOverlap(Box)
  (params (OverlappedComponent :type Primitive%20Component%20Object%20Reference) (OtherActor :type Actor%20Object%20Reference) (OtherComp :type Primitive%20Component%20Object%20Reference) (OtherBodyIndex :type Integer) (bFromSweep :type Boolean) (SweepResult :type Hit%20Result%20Structure%20%28by%20ref%29))
  (bind _asbp_third_person_character (Utilities|Casting|CastToBP_ThirdPersonCharacter OtherActor))
  (Character|LaunchCharacter _asbp_third_person_character (Math|Vector|MakeVector (.x (* (Transformation|GetActorForwardVector _asbp_third_person_character) 5e+02)) (.y (* (Transformation|GetActorForwardVector _asbp_third_person_character) 5e+02)) 5e+02) true true)
  (Default|RagdollEvent _asbp_third_person_character 1.0))

(event EventBeginPlay)

(event Collision|EventActorBeginOverlap
  (params (OtherActor :type Actor%20Object%20Reference)))

(event EventTick
  (params (DeltaSeconds :type Float%20%28single-precision%29)))

(fn ConstructionScript
  (bind _box (Variables|Default|GetBox))
  (if (Variables|Default|GetRagdollEffect)
    (Variables|/Script/Engine.PrimitiveComponent|SetbGenerateOverlapEvents _box true)
    (else
      (Variables|/Script/Engine.PrimitiveComponent|SetbGenerateOverlapEvents _box false))))